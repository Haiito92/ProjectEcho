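; BPC_StateMachine is a pawn-side Blueprint that exposes recording hooks for actions and control rotation.
; It forwards start and stop events to its RecordHandler and returns that handler's list of actions to record.
; Whether to record comes from the RecordManagerSubsystem's global recording flag.
; Control rotation is read from the pawn and written through its controller; no state machine logic appears in these graphs.
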(fn ConstructionScript)

(event EventStartRecording
  (Class|RecordHandlerComponent|StartRecording (Variables|Default|GetRecordHandler)))

(event EventStopRecording
  (Class|RecordHandlerComponent|StopRecording (Variables|Default|GetRecordHandler)))

(event EventSetControlRotation
  (params (NewControlRotation :type Rotator :default "0, 0, 0"))
  (Pawn|SetControlRotation (Pawn|GetController) NewControlRotation))

(fn GettoRecordActions
  (return (Class|RecordHandlerComponent|GettoRecordActions (Variables|Default|GetRecordHandler))))

(fn GettoRecordControlRotation
  (return (Pawn|GetControlRotation :!class /Script/Engine.Pawn)))

(fn ShouldRecord
  (return (Class|RecordManagerSubsystem|IsRecording (Subsystems|GetRecordManagerSubsystem))))

(fn ConstructionScript)
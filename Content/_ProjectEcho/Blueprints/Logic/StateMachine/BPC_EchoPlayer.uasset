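; Player character Blueprint that drives echo recording and plays the player's sound effects.
; Start and stop recording forward to the RecordHandler, toggle a looping echo sound and override submix effect chains while recording.
; Tick checks velocity to run a looping footstep timer, while jump, land, death, reflect and grab events spawn attached sounds.
; Small functions expose control rotation and recording state to the record system.
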(event OnReflectStarted(BP_ReflectComponent)
  ;[0.01681 0.107 0.15 0.502] React to player reflect component events
  (bind _returnvalue (Audio|SpawnSoundAttached "/Game/_ProjectEcho/Assets/Audio/MSSource/MC/Push/MSS_MC_Push_Charge.MSS_MC_Push_Charge" (Variables|Default|GetCapsuleComponent) "None" "0, 0, 0" "0, 0, 0" "KeepRelativeOffset" false 1.0 1.0 0.0 0 0))
  (Variables|Default|SetPushChargeSFX _returnvalue))

(event OnObjectReflected(BP_ReflectComponent)
  (bind _pushchargesfx (Variables|Default|GetPushChargeSFX))
  ;[0.01681 0.107 0.15 0.502] React to player reflect component events
  (Utilities|IsValid _pushchargesfx
    (:Is%20Valid
      (Class|AudioParameterControllerInterface|SetTriggerParameter _pushchargesfx "Stop"))
    (:Is%20Not%20Valid
      _))
  (Audio|SpawnSoundAttached "/Game/_ProjectEcho/Assets/Audio/MSSource/MC/Push/MSS_MC_Push_Activate.MSS_MC_Push_Activate" (Variables|Default|GetCapsuleComponent) "None" "0, 0, 0" "0, 0, 0" "KeepRelativeOffset" false 1.0 1.0 0.0 0 0))

(event OnReflectStopped(BP_ReflectComponent)
  (bind _pushchargesfx (Variables|Default|GetPushChargeSFX))
  ;[0.01681 0.107 0.15 0.502] React to player reflect component events
  (Utilities|IsValid _pushchargesfx
    (:Is%20Valid
      (Class|AudioParameterControllerInterface|SetTriggerParameter _pushchargesfx "Stop"))))

(event OnActorGrabbed(Grabbing)
  (params (GrabActor :type Actor%20Object%20Reference))
  ;[0.03776 0.15 0.06293 0.5] React to player grab component events
  (Audio|SpawnSoundAttached "/Game/_ProjectEcho/Assets/Audio/MSSource/MC/PickUp/MSS_MC_PickUp.MSS_MC_Pickup" (Variables|Default|GetCapsuleComponent) "None" "0, 0, 0" "0, 0, 0" "KeepRelativeOffset" false 1.0 1.0 0.0 0 0))

(event OnActorReleased(Grabbing)
  ;[0.03776 0.15 0.06293 0.5] React to player grab component events
  (Audio|SpawnSoundAttached "/Game/_ProjectEcho/Assets/Audio/MSSource/MC/Release/MSS_MC_Release.MSS_MC_Release" (Variables|Default|GetCapsuleComponent) "None" "0, 0, 0" "0, 0, 0" "KeepRelativeOffset" false 1.0 1.0 0.0 0 0))

(event OnActorThrowed(Grabbing)
  ;[0.03776 0.15 0.06293 0.5] React to player grab component events
  (Audio|SpawnSoundAttached "/Game/_ProjectEcho/Assets/Audio/MSSource/MC/Launch/MSS_MC_Launch.MSS_MC_Launch" (Variables|Default|GetCapsuleComponent) "None" "0, 0, 0" "0, 0, 0" "KeepRelativeOffset" false 1.0 1.0 0.0 0 0))

(event Custom|OnChangeState_Event
  (params (newState :type EState%20Enum :default "Idle"))
  (Variables|Default|SetNew%20State newState))

(event Custom|FT
  (bind _capsulecomponent (Variables|Default|GetCapsuleComponent))
  ;[0.9375 0.1367 0.713 0.5] Footstep SFX
  ;;[0.1303 0.8073 0.2537 0.5] Play Footstep and foley every X seconds
  (Audio|SpawnSoundAttached "/Game/_ProjectEcho/Assets/Audio/MSSource/MC/FT/Walk/MSS_MC_FT_Walk_Concrete.MSS_MC_FT_Walk_Concrete" _capsulecomponent "None" "0, 0, 0" "0, 0, 0" "KeepRelativeOffset" false 1.0 1.0 0.0 0 0)
  (Audio|SpawnSoundAttached "/Game/_ProjectEcho/Assets/Audio/MSSource/MC/FOL/Walk/MSS_MC_FOL_Walk.MSS_MC_FOL_Walk" _capsulecomponent "None" "0, 0, 0" "0, 0, 0" "KeepRelativeOffset" false 1.0 1.0 0.0 0 0))

(event EventBeginPlay
  (EventDispatchers|AssignOnChangeState (Variables|Default|GetStateMachine) (delegate Custom|OnChangeState_Event))
  (CallFunction|GetAnimationBlueprint)
  (Variables|/Game/_ProjectEcho/Blueprints/Logic/ReflectMechanic/BP_ReflectComponent.BP_ReflectComponent_C|SetNiagaraSystem (Variables|Default|GetBP_ReflectComponent) (Variables|Default|GetReflectFeedbackVFX)))

(event EventOnLanded
  (params (Hit :type Hit%20Result%20Structure%20%28by%20ref%29))
  (bind _capsulecomponent (Variables|Default|GetCapsuleComponent))
  ;[0.9375 0.1367 0.713 0.5] Land SFX
  (Audio|SpawnSoundAttached "/Game/_ProjectEcho/Assets/Audio/MSSource/MC/FOL/Land/MSS_MC_FOL_Land.MSS_MC_FOL_Land" _capsulecomponent "None" "0, 0, 0" "0, 0, 0" "KeepRelativeOffset" false 1.0 1.0 0.0 0 0)
  (Audio|SpawnSoundAttached "/Game/_ProjectEcho/Assets/Audio/MSSource/MC/FT/Land/MSS_MC_FT_Land_Concrete.MSS_MC_FT_Land_Concrete" _capsulecomponent "None" "0, 0, 0" "0, 0, 0" "KeepRelativeOffset" false 1.0 1.0 0.0 0 0))

(event EventLaserize
  ;[0.15 0.02005 0.02005 0.5] Player Laserize event
)

(event EventSetControlRotation
  (params (NewControlRotation :type Rotator :default "0, 0, 0"))
  (Pawn|SetControlRotation (Pawn|GetController) NewControlRotation))

(event EventOnJumped
  (bind _capsulecomponent (Variables|Default|GetCapsuleComponent))
  ;[0.9375 0.1367 0.713 0.5] Jump SFX
  (Audio|SpawnSoundAttached "/Game/_ProjectEcho/Assets/Audio/MSSource/MC/FT/Jump/MSS_MC_FT_Jump_Concrete.MSS_MC_FT_Jump_Concrete" _capsulecomponent "None" "0, 0, 0" "0, 0, 0" "KeepRelativeOffset" false 1.0 1.0 0.0 0 0)
  (Audio|SpawnSoundAttached "/Game/_ProjectEcho/Assets/Audio/MSSource/MC/FOL/Jump/MSS_MC_FOL_Jump.MSS_MC_FOL_Jump" _capsulecomponent "None" "0, 0, 0" "0, 0, 0" "KeepRelativeOffset" false 1.0 1.0 0.0 0 0)
  (Utilities|FlowControl|Delay 0.5))

(event EventStopRecording
  (Utilities|FlowControl|Sequence
    (:then_0
      (Class|RecordHandlerComponent|StopRecording (Variables|Default|GetRecordHandler)))
    (:then_1
      ;[0.9375 0.1367 0.713 0.5] Recording SFX Stop
      (Audio|SpawnSoundAttached "/Game/_ProjectEcho/Assets/Audio/MSSource/MC/Echo/MSS_MC_Echo_Stop.MSS_MC_Echo_Stop" (Variables|Default|GetCapsuleComponent) "None" "0, 0, 0" "0, 0, 0" "KeepRelativeOffset" false 1.0 1.0 0.0 0 0)
      (Class|AudioParameterControllerInterface|SetTriggerParameter (Variables|Default|GetEchoLP) "Stop")
      ;[0.9375 0.1367 0.713 0.5] sound effects deactivation
      (Class|AudioMixerBlueprintLibrary|ClearSubmixEffectChainOverride "/Game/_ProjectEcho/Assets/Audio/Mix/Submix/Sbm_MC_FT.Sbm_MC_FT" 0.5)
      (Class|AudioMixerBlueprintLibrary|ClearSubmixEffectChainOverride "/Game/_ProjectEcho/Assets/Audio/Mix/Submix/Sbm_GPE.Sbm_GPE" 0.5)
      (Class|AudioMixerBlueprintLibrary|ClearSubmixEffectChainOverride "/Game/_ProjectEcho/Assets/Audio/Mix/Submix/Sbm_ECHOES.Sbm_ECHOES" 0.5))))

(event EventTick
  (params (DeltaSeconds :type Float%20%28single-precision%29))
  (bind _returnvalue (Game|Player|GetPlayerPawn 0))
  (bind _returnvalue_2 (Transformation|GetVelocity _returnvalue))
  ;[0.9375 0.1367 0.713 0.5] Footstep SFX
  (if (and (Math|Boolean|ORBoolean (>= (.x _returnvalue_2) 2.0) (<= (.x _returnvalue_2) -2.0) (>= (.y _returnvalue_2) 2.0) (<= (.y _returnvalue_2) -2.0)) (== (.z _returnvalue_2) 0.0))
    (Utilities|FlowControl|DoOnce false :!label _label
      (:Completed
        ;;[0.1303 0.8073 0.2537 0.5] Play Footstep and foley every X seconds
        (bind _returnvalue_3 (Utilities|Time|SetTimerbyEvent (delegate Custom|FT) 0.5 true))
        (Variables|Default|SetFTTimer _returnvalue_3)))
    (else
      (Utilities|Time|ClearandInvalidateTimerbyHandle (Variables|Default|GetFTTimer))
      (goto _label Reset))))

(event EventDeathInRecord
  ;[0.15 0.0774 0.02051 0.5] Player Death events
  (Audio|SpawnSoundAttached "/Game/_ProjectEcho/Assets/Audio/MSSource/MC/Death/MSS_MC_Death.MSS_MC_Death" (Variables|Default|GetCapsuleComponent) "None" "0, 0, 0" "0, 0, 0" "KeepRelativeOffset" false 1.0 1.0 0.0 0 0))

(event EventDeathOutOfRecord
  ;[0.15 0.0774 0.02051 0.5] Player Death events
  (Audio|SpawnSoundAttached "/Game/_ProjectEcho/Assets/Audio/MSSource/MC/Death/MSS_MC_Death.MSS_MC_Death" (Variables|Default|GetCapsuleComponent) "None" "0, 0, 0" "0, 0, 0" "KeepRelativeOffset" false 1.0 1.0 0.0 0 0))

(event EventStartRecording
  (bind _record_submix_effect_preset_chain (Variables|Default|GetRecord%20Submix%20Effect%20Preset%20Chain))
  (bind _capsulecomponent (Variables|Default|GetCapsuleComponent))
  (Utilities|FlowControl|Sequence
    (:then_0
      (Class|RecordHandlerComponent|StartRecording (Variables|Default|GetRecordHandler)))
    (:then_1
      ;[0.9375 0.1367 0.713 0.5] recording SFX start
      (Audio|SpawnSoundAttached "/Game/_ProjectEcho/Assets/Audio/MSSource/MC/Echo/MSS_MC_Echo_Start.MSS_MC_Echo_Start" _capsulecomponent "None" "0, 0, 0" "0, 0, 0" "KeepRelativeOffset" false 1.0 1.0 0.0 0 0)
      (bind _returnvalue (Audio|SpawnSoundAttached "/Game/_ProjectEcho/Assets/Audio/MSSource/MC/Echo/MSS_MC_Echo_LP.MSS_MC_Echo_LP" _capsulecomponent "None" "0, 0, 0" "0, 0, 0" "KeepRelativeOffset" false 1.0 1.0 0.0 0 0))
      (Variables|Default|SetEchoLP _returnvalue)
      ;[0.9375 0.1367 0.713 0.5] Sound effects activation on recording
      (Class|AudioMixerBlueprintLibrary|SetSubmixEffectChainOverride "/Game/_ProjectEcho/Assets/Audio/Mix/Submix/Sbm_MC_FT.Sbm_MC_FT" _record_submix_effect_preset_chain 0.0)
      (Class|AudioMixerBlueprintLibrary|SetSubmixEffectChainOverride "/Game/_ProjectEcho/Assets/Audio/Mix/Submix/Sbm_GPE.Sbm_GPE" _record_submix_effect_preset_chain 0.0)
      (Class|AudioMixerBlueprintLibrary|SetSubmixEffectChainOverride "/Game/_ProjectEcho/Assets/Audio/Mix/Submix/Sbm_ECHOES.Sbm_ECHOES" _record_submix_effect_preset_chain 0.0))))

(fn ConstructionScript)

(fn GettoRecordControlRotation
  (return (Pawn|GetControlRotation :!class /Script/Engine.Pawn)))

(fn ReceiveGetDefaultAnimationValues)

(fn GetAnimationBlueprint
  (bind _asabp_echo_create_data (Utilities|Casting|CastToABP_Echo_Create_Data (Components|SkeletalMesh|GetAnimInstance (Variables|Character|GetMesh))))
  (Variables|Default|SetABP%20Echo _asabp_echo_create_data))

(fn GetRecorderTimelineIndex
  (return 255))

(fn ShouldInteractionListenforRecord
  (return true))

(fn ShouldRecord
  (return (Class|RecordManagerSubsystem|IsRecording (Subsystems|GetRecordManagerSubsystem))))
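; Manages the main menu's in-world UI, moving the camera and keyboard focus between main and options world widgets.
; Init binds to the menu event holder and viewport focus event, initializes both widgets, and spawns dummy widget and camera actors as fallbacks.
; Menu requests blend the view target, apply that camera's FOV and focus the widget, with Pause mapped to Main.
; Regaining viewport focus restores keyboard focus to the current widget.
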(event Custom|StartWorldUI
  (Utilities|FlowControl|Delay 0.2)
  (CallFunction|FocusonWidget "MainMenu"))

(event EventTick
  (params (DeltaSeconds :type Float%20%28single-precision%29)))

(fn ConstructionScript)

(fn InitWorldUIManager
  (params (MenuEventHolder :type Menu%20Event%20Holder%20Object%20Reference) (EchoPlayerController :type Echo%20Player%20Controller%20Base%20Object%20Reference))
  (bind _returnvalue (Class|EchoGameplayStatics|GetEchoGameViewportClient))
  (Variables|Default|SetMenu%20Event%20Holder MenuEventHolder)
  (Variables|Default|SetEchoPlayerController EchoPlayerController)
  (Utilities|FlowControl|Sequence
    (:then_0
      (bind _returnvalue_2 (Game|SpawnActorfromClass "/Game/_ProjectEcho/Blueprints/Logic/MainMenu/BP_WorldWidget.BP_WorldWidget_C" (Math|Transform|MakeTransform "0, 0, 0" "0, 0, 0" "1.000000,1.000000,1.000000") "Undefined" "MultiplyWithRoot" 0 0))
      (Variables|WorldUI|Widgets|SetDummyWorldWidget _returnvalue_2)
      (bind _returnvalue_3 (Game|SpawnActorfromClass "/Game/_ProjectEcho/Blueprints/Logic/MainMenu/BP_WorldMenuCamPos.BP_WorldMenuCamPos_C" (Math|Transform|MakeTransform "0, 0, 0" "0, 0, 0" "1.000000,1.000000,1.000000") "Undefined" "MultiplyWithRoot" 0 0))
      (Variables|WorldUI|CamPos|SetDummyCamPos _returnvalue_3))
    (:then_1
      (bind _menu_event_holder (Variables|Default|GetMenu%20Event%20Holder)
        (:then
          (EventDispatchers|BindEventtoOnGotoMenuPressed _menu_event_holder (EventDispatchers|CreateEvent :!event OnGotoMenuPressed)))
        (:else
          (Class|EchoDebug|LogandAddonScreenDebugMessage "GameLoop" "Error" "World UI Manager: Invalid Menu Event Handler" "(R=1.000000,G=0.167654,B=0.070055,A=1.000000)" 3.0)))
      (Utilities|IsValid _returnvalue
        (:Is%20Valid
          (EventDispatchers|BindEventtoOnViewportReceivedFocus _returnvalue (EventDispatchers|CreateEvent :!event BPonViewportReceivedFocus)))
        (:Is%20Not%20Valid
          (Class|EchoDebug|LogandAddonScreenDebugMessage "GameLoop" "Error" "World UI Manager: Invalid Echo Game Viewport Client" "(R=1.000000,G=0.167654,B=0.070055,A=1.000000)" 3.0))))
    (:then_2
      (bind _mainmenuworldwidget (Variables|WorldUI|Widgets|GetMainMenuWorldWidget)
        (:then
          (Class|BPIEchoWidget|InitEchoWidget(Message) _mainmenuworldwidget (Variables|Default|GetMenu%20Event%20Holder)))
        (:else)))
    (:then_3
      (bind _optionsworldwidget (Variables|WorldUI|Widgets|GetOptionsWorldWidget)
        (:then
          (bind _aswbp_options_menu (Utilities|Casting|CastToWBP_OptionsMenu (UserInterface|GetWidget (Variables|/Game/_ProjectEcho/Blueprints/Logic/MainMenu/BP_WorldWidget.BP_WorldWidget_C|GetWidgetComponent _optionsworldwidget)))
            (:then
              (Default|InitOptionsMenu _aswbp_options_menu (Variables|Default|GetMenu%20Event%20Holder) "MainMenu"))
            (:CastFailed
              (Class|BPIEchoWidget|InitEchoWidget(Message) _optionsworldwidget (Variables|Default|GetMenu%20Event%20Holder)))))
        (:else)))))

(fn FocusonWidget
  (params (MenuType :type MenuType%20Enum :default "MainMenu"))
  (bind _dummyworldwidget (Variables|WorldUI|Widgets|GetDummyWorldWidget))
  (bind _optionsworldwidget (Variables|WorldUI|Widgets|GetOptionsWorldWidget))
  (bind _dummyworldwidget_2 (Variables|WorldUI|Widgets|GetDummyWorldWidget))
  (bind _dummycampos (Variables|WorldUI|CamPos|GetDummyCamPos))
  (bind _dummycampos_2 (Variables|WorldUI|CamPos|GetDummyCamPos))
  (bind _mainmenucampos (Variables|WorldUI|CamPos|GetMainMenuCamPos))
  (bind _optionscampos (Variables|WorldUI|CamPos|GetOptionsCamPos))
  (bind _mainmenuworldwidget (Variables|WorldUI|Widgets|GetMainMenuWorldWidget))
  (bind _returnvalue (Utilities|IsValid _optionsworldwidget))
  (bind _returnvalue_2 (Utilities|IsValid _mainmenuworldwidget))
  (bind _returnvalue_3 (Utilities|IsValid _mainmenucampos))
  (bind _returnvalue_4 (Utilities|IsValid _optionscampos))
  (bind _returnvalue_5 (select _returnvalue _optionsworldwidget _dummyworldwidget))
  (bind _returnvalue_6 (select _returnvalue_2 _mainmenuworldwidget _dummyworldwidget_2))
  (bind _returnvalue_7 (select _returnvalue_3 _mainmenucampos _dummycampos_2))
  (bind _returnvalue_8 (select _returnvalue_4 _optionscampos _dummycampos))
  (bind _returnvalue_9 (Utilities|Select :Index MenuType :MainMenu _returnvalue_7 :OptionsMenu _returnvalue_8 :PauseMenu _returnvalue_7))
  (bind _returnvalue_10 (Utilities|Select :Index MenuType :MainMenu _returnvalue_6 :OptionsMenu _returnvalue_5 :PauseMenu _returnvalue_6))
  (bind _echoplayercontroller (Variables|Default|GetEchoPlayerController)
    (:then
      (Game|Player|SetViewTargetwithBlend _echoplayercontroller _returnvalue_9 (Variables|WorldUI|CamPos|GetCamBlendTime) "VTBlend_Linear" 0.0 false)
      (Variables|/Script/Engine.PlayerCameraManager|SetDefaultFOV (Variables|/Script/Engine.PlayerController|GetPlayerCameraManager (Variables|Default|GetEchoPlayerController)) (Variables|/Game/_ProjectEcho/Blueprints/Logic/MainMenu/BP_WorldMenuCamPos.BP_WorldMenuCamPos_C|GetFov _returnvalue_9)))
    (:else
      _))
  (Class|BPIEchoWidget|SetKeyboardFocusonWidget(Message) _returnvalue_10)
  (Variables|WorldUI|Widgets|SetCurrentFocusedWorldWidget _returnvalue_10))

(fn OnGotoMenuPressed
  (params (MenuType :type MenuType%20Enum :default "MainMenu"))
  (CallFunction|FocusonWidget MenuType))

(fn BPonViewportReceivedFocus
  (bind _currentfocusedworldwidget (Variables|WorldUI|Widgets|GetCurrentFocusedWorldWidget))
  (Utilities|IsValid _currentfocusedworldwidget
    (:Is%20Valid
      (Class|BPIEchoWidget|SetKeyboardFocusonWidget(Message) _currentfocusedworldwidget))))
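; BP_Lever is a timed lever level-design element that switches on when interacted with and switches itself off after SwitchedOnTime.
; Interact drives an activator component and starts the timer, ignoring presses while the lever is already on.
; The component's on and off events flip the handle rotation and play activate and deactivate sounds.
; A looping MetaSound runs while the lever is on and is stopped through a trigger parameter.
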(event OnActivatorSwitchedon(BP_ActivatorComponent)
  (Transformation|SetRelativeRotation (Variables|Default|GetLeverHandle) "-40.000000,0.000000,0.000000" false false)
  ;[0.9375 0.1367 0.713 0.5] Lever SFX
  (Audio|SpawnSoundAttached "/Game/_ProjectEcho/Assets/Audio/MSSource/GPE/Lever/MSS_GPE_Lever_Activate.MSS_GPE_Lever_Activate" (Variables|Default|GetBase) "None" "0, 0, 0" "0, 0, 0" "KeepRelativeOffset" false 1.0 1.0 0.0 0 0)
  (bind _returnvalue (Audio|SpawnSoundAttached "/Game/_ProjectEcho/Assets/Audio/MSSource/GPE/Lever/MSS_GPE_Lever_LP.MSS_GPE_Lever_LP" (Variables|Default|GetBase) "None" "0, 0, 0" "0, 0, 0" "KeepRelativeOffset" false 1.0 1.0 0.0 0 0))
  (Variables|Default|SetLeverLP _returnvalue))

(event OnActivatorSwitchedOff(BP_ActivatorComponent)
  (bind _leverlp (Variables|Default|GetLeverLP))
  (Transformation|SetRelativeRotation (Variables|Default|GetLeverHandle) "40.000000,0.000000,0.000000" false false)
  ;[0.9375 0.1367 0.713 0.5] Lever SFX
  (Audio|SpawnSoundAttached "/Game/_ProjectEcho/Assets/Audio/MSSource/GPE/Lever/MSS_GPE_Lever_Deactivate.MSS_GPE_Lever_Deactivate" (Variables|Default|GetBase) "None" "0, 0, 0" "0, 0, 0" "KeepRelativeOffset" false 1.0 1.0 0.0 0 0)
  (if (Utilities|IsValid _leverlp)
    (Class|AudioParameterControllerInterface|SetTriggerParameter _leverlp "Stop")))

(event Custom|CE_OnLeverTimerElapsed
  (bind _bp_activatorcomponent (Variables|Default|GetBP_ActivatorComponent))
  (bind _returnvalue (Class|Activator|IsSwitchon _bp_activatorcomponent))
  (if _returnvalue
    (Class|Activator|SwitchOff _bp_activatorcomponent)))

(event EventBeginPlay
  (Transformation|SetRelativeRotation (Variables|Default|GetLeverHandle) "40.000000,0.000000,0.000000" false false))

(event EventInteract
  (bind _bp_activatorcomponent (Variables|Default|GetBP_ActivatorComponent))
  (bind _returnvalue (Class|Activator|IsSwitchon _bp_activatorcomponent))
  (if (not _returnvalue)
    (Class|Activator|Switchon _bp_activatorcomponent)
    (Utilities|Time|SetTimerbyEvent (delegate Custom|CE_OnLeverTimerElapsed) (Variables|Lever|GetSwitchedOnTime))))

(fn ConstructionScript)
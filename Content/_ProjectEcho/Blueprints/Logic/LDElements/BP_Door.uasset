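; BP_Door is a level-design door that slides vertically between its placed position and an offset when activated or deactivated.
; Activate and Deactivate call Open and Close, which play or reverse a timeline.
; The timeline's offset track, scaled by MaxZOffset, drives a swept move from the stored start location, with play rate derived from AnimationLength.
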(event Custom|Open
  (bind _offsettrack (Timeline|DoorTimeline Play)
    (:Update
      (Transformation|SetActorLocation (+ (Variables|Default|GetStartPos) (Math|Vector|MakeVector 0.0 0.0 (* _offsettrack (Variables|Default|GetMaxZOffset)))) true false))))

(event Custom|Close
  (bind _offsettrack (Timeline|DoorTimeline Reverse)
    (:Update
      (Transformation|SetActorLocation (+ (Variables|Default|GetStartPos) (Math|Vector|MakeVector 0.0 0.0 (* _offsettrack (Variables|Default|GetMaxZOffset)))) true false))))

(event EventActivate
  (CallFunction|Open))

(event EventDeactivate
  (CallFunction|Close))

(event EventBeginPlay
  (Variables|Default|SetStartPos (Transformation|GetActorLocation))
  (Components|Timeline|SetPlayRate (Variables|Default|GetDoorTimeline) (/ 1.0 (Variables|Default|GetAnimationLength))))

(fn ConstructionScript)
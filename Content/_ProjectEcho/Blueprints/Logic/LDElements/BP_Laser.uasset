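; BP_Laser is a level-design hazard that fires a straight laser along the actor's forward vector and kills what it hits.
; Every tick, ShootLaser sphere-traces WorldStatic and WorldDynamic objects over a configurable distance and radius, sending KillMessage to a blocking hit actor implementing Killable.
; It redraws the beam in red as a line capped by spheres, shortened to the hit point when blocked, using draw calls keyed to Activable.
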(event EventTick
  (params (DeltaSeconds :type Float%20%28single-precision%29))
  (CallFunction|ShootLaser))

(fn ConstructionScript)

(fn ShootLaser
  (LocalVariables|SetFinalDistance (Math|Float|Max(Float) (Variables|Default|GetMaxDistance) 0.0))
  (LocalVariables|SetFinalRadius (Math|Float|Max(Float) (Variables|Default|GetRadius) 0.0))
  (bind _output_get (LocalVariables|SetStartPoint (Transformation|GetWorldLocation (Variables|Default|GetScene))))
  (LocalVariables|SetEndPoint (+ _output_get (* (Transformation|GetActorForwardVector) (LocalVariables|GetFinalDistance))))
  (Utilities|FlowControl|Sequence
    (:then_0
      (bind _outhit (Collision|SphereTraceForObjects (LocalVariables|GetStartPoint) (LocalVariables|GetEndPoint) (LocalVariables|GetFinalRadius) (Utilities|Array|MakeArray "ObjectTypeQuery1" "ObjectTypeQuery2") false 0 "None"))
      (if (.bBlockingHit (Collision|BreakHitResult _outhit))
        (if (Utilities|DoesObjectImplementInterface (.HitActor (Collision|BreakHitResult _outhit)) "/Script/ProjectEcho.Killable")
          (Class|Killable|Kill(Message) (.HitActor (Collision|BreakHitResult _outhit))))))
    (:then_1
      (Class|EchoDebug|DrawSphere "Activable" (LocalVariables|GetStartPoint) (LocalVariables|GetFinalRadius) 12 "(R=1.000000,G=0.079664,B=0.033808,A=1.000000)" 0.0 0.0 "World")
      (if (.bBlockingHit (Collision|BreakHitResult _outhit))
        (Class|EchoDebug|DrawLine "Activable" (LocalVariables|GetStartPoint) (.Location (Collision|BreakHitResult _outhit)) "(R=1.000000,G=0.080220,B=0.034340,A=1.000000)" 0.0 0.0 "World")
        (Class|EchoDebug|DrawSphere "Activable" (.Location (Collision|BreakHitResult _outhit)) (LocalVariables|GetFinalRadius) 12 "(R=1.000000,G=0.079664,B=0.033808,A=1.000000)" 0.0 0.0 "World")
        (else
          (Class|EchoDebug|DrawLine "Activable" (LocalVariables|GetStartPoint) (LocalVariables|GetEndPoint) "(R=1.000000,G=0.080220,B=0.034340,A=1.000000)" 0.0 0.0 "World")
          (Class|EchoDebug|DrawSphere "Activable" (LocalVariables|GetEndPoint) (LocalVariables|GetFinalRadius) 12 "(R=1.000000,G=0.079664,B=0.033808,A=1.000000)" 0.0 0.0 "World"))))))
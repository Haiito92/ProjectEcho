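; Physics cube that can be grabbed, released or thrown, and works with the record and rewind system.
; Grabbing disables physics and collision and notifies the Recordable component, using the grabber's record flag if available.
; Rewind callbacks suspend and restore physics while clearing velocities.
; Kill returns it to its BeginPlay transform, while Reset, also on NumPad 9, restores location, zeroes rotation and disables physics.
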(event Custom|OnStartRewind
  (bind _cube (Variables|Default|GetCube))
  (Physics|SetSimulatePhysics _cube false)
  (Physics|SetPhysicsLinearVelocity _cube "0, 0, 0" false "None")
  (Class|PrimitiveComponent|SetPhysicsAngularVelocityinDegrees _cube "0, 0, 0" false "None"))

(event Custom|OnStopRewind
  (bind _cube (Variables|Default|GetCube))
  (Physics|SetSimulatePhysics _cube true)
  (Physics|SetPhysicsLinearVelocity _cube "0, 0, 0" false "None")
  (Class|PrimitiveComponent|SetPhysicsAngularVelocityinDegrees _cube "0, 0, 0" false "None"))

(event Custom|Reset
  (Physics|SetSimulatePhysics (Variables|Default|GetCube) false)
  (Transformation|SetActorLocation (Variables|Default|GetDefaultLocation) false true)
  (Transformation|SetActorRotation "0, 0, 0" true))

(event EventBeginPlay
  (bind _recordable (Variables|Default|GetRecordable))
  (Variables|Default|SetDefaultLocation (Transformation|GetActorLocation))
  (Variables|Default|SetDefaultRotation (Transformation|GetActorRotation))
  (EventDispatchers|BindEventtoOnStartRewind _recordable (EventDispatchers|CreateEvent :!event Custom|OnStartRewind))
  (EventDispatchers|BindEventtoOnStopRewind _recordable (EventDispatchers|CreateEvent :!event Custom|OnStopRewind)))

(event EventKill
  (bind _cube (Variables|Default|GetCube))
  ;[0.15 0.15 0.15 0.5] Killable
  (Physics|SetPhysicsLinearVelocity _cube "0, 0, 0" false "None")
  (Class|PrimitiveComponent|SetPhysicsAngularVelocityinDegrees _cube "0, 0, 0" false "None")
  (Transformation|SetActorLocationAndRotation (Variables|Default|GetDefaultLocation) (Variables|Default|GetDefaultRotation)))

(event EventTick
  (params (DeltaSeconds :type Float%20%28single-precision%29)))

(event EventOnBeforeGrabbed
  (params (GrabbingActor :type Actor%20Object%20Reference))
  (bind _cube (Variables|Default|GetCube))
  (bind _recordable (Variables|Default|GetRecordable))
  (bind _recordable_2 (Variables|Default|GetRecordable))
  (Utilities|FlowControl|Sequence
    (:then_0
      (Physics|SetSimulatePhysics _cube false)
      (Collision|SetCollisionEnabled _cube "NoCollision"))
    (:then_1
      (if (Utilities|DoesObjectImplementInterface GrabbingActor "/Script/ProjectEcho.IRecordInteractorInterface")
        (bind _returnvalue (Class|IRecordInteractorInterface|ShouldRecord(Message) GrabbingActor))
        (Default|CallOnInteracted _recordable _recordable _returnvalue)
        (else
          (Default|CallOnInteracted _recordable_2 _recordable_2 false))))))

(event EventOnThrown
  (params (ThrowDirection :type Vector%20%28by%20ref%29 :default "0, 0, 0") (ThrowForce :type Float%20%28single-precision%29%20%28by%20ref%29))
  (bind _cube (Variables|Default|GetCube))
  (Utilities|FlowControl|Sequence
    (:then_0
      (Physics|SetSimulatePhysics _cube true)
      (Collision|SetCollisionEnabled _cube "QueryAndPhysics"))
    (:then_1
      (Physics|AddImpulse (Variables|Default|GetCube) (* ThrowDirection ThrowForce) "None" true))))

(event EventOnObjectReleased
  (bind _cube (Variables|Default|GetCube))
  (Physics|SetSimulatePhysics _cube true)
  (Collision|SetCollisionEnabled _cube "QueryAndPhysics"))

(event Input|KeyboardEvents|NumPadNine
  (params (Key :type Key%20Structure :default "None"))
  (:Pressed
    (Physics|SetSimulatePhysics (Variables|Default|GetCube) false)
    (Transformation|SetActorLocation (Variables|Default|GetDefaultLocation) false true)
    (Transformation|SetActorRotation "0, 0, 0" true)))

(fn ConstructionScript)

(fn CanbeGrabbed
  (return true))
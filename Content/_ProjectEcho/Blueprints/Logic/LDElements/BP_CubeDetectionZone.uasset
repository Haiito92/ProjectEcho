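; BP_CubeDetectionZone is a level-design trigger zone that turns its activator on while cubes are inside it.
; It counts overlapping actors that implement the Cube interface, raising the count on begin overlap and lowering it on end overlap, clamped at zero.
; The BPActivatorComponent switches on when the count rises to one and off when the count is zero after a cube leaves.
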(event Collision|EventActorBeginOverlap
  (params (OtherActor :type Actor%20Object%20Reference))
  (if (Utilities|DoesObjectImplementInterface OtherActor "/Script/ProjectEcho.Cube")
    (bind _result (Math|Integer|IncrementInt (Variables|Default|GetCubeCount))
      (:%20%20
        (if (== _result 1)
          (Class|Activator|Switchon (Variables|Default|GetBP_ActivatorComponent)))))))

(event Collision|EventActorEndOverlap
  (params (OtherActor :type Actor%20Object%20Reference))
  (if (Utilities|DoesObjectImplementInterface OtherActor "/Script/ProjectEcho.Cube")
    (bind _output_get (Variables|Default|SetCubeCount (Math|Integer|Max(Integer) (- (Variables|Default|GetCubeCount) 1))))
    (if (== 0 _output_get)
      (Class|Activator|SwitchOff (Variables|Default|GetBP_ActivatorComponent)))))

(fn ConstructionScript)
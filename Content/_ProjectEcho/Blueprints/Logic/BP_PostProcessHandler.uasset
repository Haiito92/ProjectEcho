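; BP_PostProcessHandler drives the recording post-process feedback by writing to the RecordMPC material parameter collection.
; On BeginPlay it binds to the RecordManagerSubsystem's start and stop recording events.
; Starting sets the collection's Color to the echo's vignette color and Activated to one; stopping clears both.
; Updates are purely event-driven, with no Tick logic and no direct reference to post-process volumes or materials.
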(event Custom|OnStartRecording
  (params (CurrentTimeKey :type Float%20%28single-precision%29) (TimelineIndex :type Integer) (EchoColorInformations :type Echo%20Color%20Struct%20Structure%20%28by%20ref%29))
  (bind _recordmpc (Variables|Default|GetRecordMPC))
  (Rendering|Material|SetVectorParameterValue _recordmpc (Utilities|Name|MakeLiteralName "Color") (Math|Conversions|ToLinearColor(Color) (.VignetteColor (Utilities|Struct|BreakEchoColorStruct EchoColorInformations))) :!class /Script/Engine.KismetMaterialLibrary)
  (Rendering|Material|SetScalarParameterValue _recordmpc (Utilities|Name|MakeLiteralName "Activated") 1.0 :!class /Script/Engine.KismetMaterialLibrary))

(event Custom|OnStopRecording
  (bind _recordmpc (Variables|Default|GetRecordMPC))
  (Rendering|Material|SetVectorParameterValue _recordmpc (Utilities|Name|MakeLiteralName "Color") (Math|Color|MakeColor 0.0 0.0 0.0 0.0) :!class /Script/Engine.KismetMaterialLibrary)
  (Rendering|Material|SetScalarParameterValue _recordmpc (Utilities|Name|MakeLiteralName "Activated") 0.0 :!class /Script/Engine.KismetMaterialLibrary))

(event EventBeginPlay
  (bind _returnvalue (Subsystems|GetRecordManagerSubsystem))
  (EventDispatchers|BindEventtoOnStartRecording _returnvalue (EventDispatchers|CreateEvent :!event Custom|OnStartRecording))
  (EventDispatchers|BindEventtoOnStopRecording _returnvalue (EventDispatchers|CreateEvent :!event Custom|OnStopRecording)))

(event Collision|EventActorBeginOverlap
  (params (OtherActor :type Actor%20Object%20Reference)))

(event EventTick
  (params (DeltaSeconds :type Float%20%28single-precision%29)))

(fn ConstructionScript)
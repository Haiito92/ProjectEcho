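; BP_AnamorphoseZoneAdapter links grabbable cubes to cube detection zones in the anamorphose logic, toggling the zones' decals while a cube is held.
; On BeginPlay it binds its handlers to the grabbed and released events of each valid cube in its Cube array.
; Any grab activates decals on every valid zone in CubeDetectionZone, and any release deactivates them all, with no per-cube pairing or held count.
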(event Custom|OnCubeGrabbed
  (for _array_element (Variables|Default|GetCubeDetectionZone)
    (Utilities|IsValid _array_element
      (:Is%20Valid
        (Default|ActivateDecals _array_element true)))))

(event Custom|OnCubeReleased
  (for _array_element (Variables|Default|GetCubeDetectionZone)
    (Utilities|IsValid _array_element
      (:Is%20Valid
        (Default|ActivateDecals _array_element false)))))

(event EventBeginPlay
  (for _array_element (Variables|Default|GetCube)
    (Utilities|IsValid _array_element
      (:Is%20Valid
        (EventDispatchers|BindEventtoOnCubeGrabbed _array_element (delegate Custom|OnCubeGrabbed))
        (EventDispatchers|BindEventtoOnCubeReleased _array_element (delegate Custom|OnCubeReleased))))))

(fn ConstructionScript)
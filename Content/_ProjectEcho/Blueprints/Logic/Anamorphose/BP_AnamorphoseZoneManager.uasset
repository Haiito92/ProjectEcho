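; Manager for an anamorphosis zone that shows detection-zone decals while its associated cube is held.
; On BeginPlay it binds to the Cube's grabbed and released events.
; Those handlers activate the CubeDetectionZone's decals on grab and deactivate them on release, with validity checks on both references.
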(event Custom|OnCubeGrabbed
  (bind _cubedetectionzone (Variables|Default|GetCubeDetectionZone))
  (Utilities|IsValid _cubedetectionzone
    (:Is%20Valid
      (Default|ActivateDecals _cubedetectionzone true))))

(event Custom|OnCubeReleased
  (bind _cubedetectionzone (Variables|Default|GetCubeDetectionZone))
  (Utilities|IsValid _cubedetectionzone
    (:Is%20Valid
      (Default|ActivateDecals _cubedetectionzone false))))

(event EventBeginPlay
  (bind _cube (Variables|Default|GetCube))
  (Utilities|IsValid _cube
    (:Is%20Valid
      (EventDispatchers|BindEventtoOnCubeGrabbed _cube (delegate Custom|OnCubeGrabbed))
      (EventDispatchers|BindEventtoOnCubeReleased _cube (delegate Custom|OnCubeReleased)))))

(fn ConstructionScript)
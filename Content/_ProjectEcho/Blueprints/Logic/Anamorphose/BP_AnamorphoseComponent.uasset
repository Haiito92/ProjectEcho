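; Decal component for anamorphosis that animates its world scale between its default and activated sizes when toggled on or off.
; On BeginPlay it picks a random decal material unless a set material is used, and creates a paused looping timer.
; Activation calls unpause the timer, which steps a clamped, curve-shaped lerp in either direction and pauses again at the target.
; A one-shot duration override can replace the normal activation time.
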(event EventBeginPlay
  (Variables|ActivationParameters|SetDefaultScale (Transformation|GetWorldScale))
  (bind _returnvalue (Utilities|Time|SetTimerbyFunctionName 0 "UpdateActivation" (Variables|ActivationParameters|GetActivationUpdateFrequency) true))
  (bind _output_get (Variables|Default|SetActivationTimer _returnvalue))
  (Utilities|Time|PauseTimerbyHandle _output_get)
  (if (not (Variables|Materials|GetUseSetMaterial))
    (Rendering|Components|Decal|SetDecalMaterial (.OutItem (Utilities|Array|Random (Variables|Materials|GetRandomMaterials))))))

(fn UpdateActivation
  (bind _result (CallFunction|SetScaletoLerpValue (+ (Variables|Default|GetActivationLerp) (Utilities|Operators|Divide (Variables|ActivationParameters|GetActivationUpdateFrequency) (Math|Float|SelectFloat (Variables|Default|GetAnimationTimeOverride) (Variables|ActivationParameters|GetActivationTime) (Variables|Default|GetActiveTimeOverride)) (Math|Float|SelectFloat 1.0 -1.0 (Variables|Default|GetIsActivated))))))
  (if (Math|Float|NearlyEqual(Float) _result (Math|Float|SelectFloat 1.0 0.0 (Variables|Default|GetIsActivated)) 0.01)
    (Transformation|SetWorldScale3D (Math|Vector|SelectVector (Variables|ActivationParameters|GetActivatedScale) (Variables|ActivationParameters|GetDefaultScale) (Variables|Default|GetIsActivated)))
    (Variables|Default|SetActiveTimeOverride false)
    (Utilities|Time|PauseTimerbyHandle (Variables|Default|GetActivationTimer))))

(fn ActivateDecal
  (params (IsActive :type Boolean))
  (bind _activationtimer (Variables|Default|GetActivationTimer))
  (Variables|Default|SetIsActivated IsActive)
  (if (Class|KismetSystemLibrary|IsTimerPausedHandle _activationtimer)
    (Utilities|Time|UnpauseTimerbyHandle _activationtimer)))

(fn ActivateDecalwithCustomActivationTime
  (params (IsActive :type Boolean) (OverrideAnimationTime :type Float%20%28double-precision%29))
  (Variables|Default|SetActiveTimeOverride true)
  (Variables|Default|SetAnimationTimeOverride OverrideAnimationTime)
  (CallFunction|ActivateDecal IsActive)
  (return))

(fn SetScaletoLerpValue
  (params (LerpValue :type Float%20%28double-precision%29))
  (bind _output_get (Variables|Default|SetActivationLerp (Math|Float|Clamp(Float) LerpValue)))
  (Transformation|SetWorldScale3D (Math|Vector|Lerp(Vector) (Variables|ActivationParameters|GetDefaultScale) (Variables|ActivationParameters|GetActivatedScale) (Math|Curves|GetFloatValue (Variables|ActivationParameters|GetActivationCurve) _output_get)))
  (return _output_get))
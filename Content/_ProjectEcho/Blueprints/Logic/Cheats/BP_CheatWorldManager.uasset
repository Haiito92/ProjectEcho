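; BP_CheatWorldManager is a debug cheat actor that teleports the player character to one of nine preset points.
; AZERTY number-row keys and numpad keys trigger the teleports when cheats are enabled and none is already running.
; InitCheatManager stores the player references and creates the load screen widget, whose fade-finished callbacks sequence each teleport.
; Player actions lock, the screen fades in, the character moves, then the screen fades out and actions unlock.
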(event Custom|TeleportToPoint
  (params (TeleportPoint :type BP%20Cheat%20Teleport%20Point%20Object%20Reference))
  (if (Math|Boolean|ANDBoolean (Variables|Cheats|GetCheatsOn) (not (Variables|Cheats|Teleport|GetOnGoingTeleport)) (Utilities|IsValid (Variables|Cheats|GetEchoPlayerCharacter)) (Utilities|IsValid TeleportPoint))
    (Variables|Cheats|Teleport|SetOnGoingTeleport true)
    (Class|CharacterST|LockAllActions (Variables|Cheats|GetEchoPlayerCharacter))
    (Variables|Cheats|Teleport|SetCurrentTeleportPoint TeleportPoint)
    (Default|CEFadein (Variables|Cheats|GetLoadScreen))))

(event Custom|CE_OnLoadScreenFadeInFinished
  (bind _currentteleportpoint (Variables|Cheats|Teleport|GetCurrentTeleportPoint))
  (Transformation|SetActorTransform (Variables|Cheats|GetEchoPlayerCharacter) (Math|Transform|MakeTransform (Transformation|GetActorLocation _currentteleportpoint) (Transformation|GetActorRotation _currentteleportpoint) "1.000000,1.000000,1.000000"))
  (Default|CEFadeOut (Variables|Cheats|GetLoadScreen)))

(event Custom|CE_OnLoadScreenFadeOutFinished
  (Class|CharacterST|UnlockAllActions (Variables|Cheats|GetEchoPlayerCharacter))
  (Variables|Cheats|Teleport|SetOnGoingTeleport false))

(event Input|KeyboardEvents|NumPadOne
  (params (Key :type Key%20Structure :default "None"))
  (:Pressed
    (CallFunction|TeleporttoPoint (Variables|Cheats|Teleport|GetTeleportPoint1))))

(event Input|KeyboardEvents|NumPadTwo
  (params (Key :type Key%20Structure :default "None"))
  (:Pressed
    (CallFunction|TeleporttoPoint (Variables|Cheats|Teleport|GetTeleportPoint2))))

(event Input|KeyboardEvents|Ampersand
  (params (Key :type Key%20Structure :default "None"))
  (:Pressed
    (CallFunction|TeleporttoPoint (Variables|Cheats|Teleport|GetTeleportPoint1))))

(event Input|KeyboardEvents|EAccentAigu
  (params (Key :type Key%20Structure :default "None"))
  (:Pressed
    (CallFunction|TeleporttoPoint (Variables|Cheats|Teleport|GetTeleportPoint2))))

(event Input|KeyboardEvents|Apostrophe
  (params (Key :type Key%20Structure :default "None"))
  (:Pressed
    (CallFunction|TeleporttoPoint (Variables|Cheats|Teleport|GetTeleportPoint4))))

(event Input|KeyboardEvents|Quote
  (params (Key :type Key%20Structure :default "None"))
  (:Pressed
    (CallFunction|TeleporttoPoint (Variables|Cheats|Teleport|GetTeleportPoint3))))

(event Input|KeyboardEvents|LeftParantheses
  (params (Key :type Key%20Structure :default "None"))
  (:Pressed
    (CallFunction|TeleporttoPoint (Variables|Cheats|Teleport|GetTeleportPoint5))))

(event Input|KeyboardEvents|EAccentGrave
  (params (Key :type Key%20Structure :default "None"))
  (:Pressed
    (CallFunction|TeleporttoPoint (Variables|Cheats|Teleport|GetTeleportPoint7))))

(event Input|KeyboardEvents|Hyphen
  (params (Key :type Key%20Structure :default "None"))
  (:Pressed
    (CallFunction|TeleporttoPoint (Variables|Cheats|Teleport|GetTeleportPoint6))))

(event Input|KeyboardEvents|Underscore
  (params (Key :type Key%20Structure :default "None"))
  (:Pressed
    (CallFunction|TeleporttoPoint (Variables|Cheats|Teleport|GetTeleportPoint8))))

(event Input|KeyboardEvents|CCedille
  (params (Key :type Key%20Structure :default "None"))
  (:Pressed
    (CallFunction|TeleporttoPoint (Variables|Cheats|Teleport|GetTeleportPoint9))))

(event Input|KeyboardEvents|NumPadThree
  (params (Key :type Key%20Structure :default "None"))
  (:Pressed
    (CallFunction|TeleporttoPoint (Variables|Cheats|Teleport|GetTeleportPoint3))))

(event Input|KeyboardEvents|NumPadFour
  (params (Key :type Key%20Structure :default "None"))
  (:Pressed
    (CallFunction|TeleporttoPoint (Variables|Cheats|Teleport|GetTeleportPoint4))))

(event Input|KeyboardEvents|NumPadFive
  (params (Key :type Key%20Structure :default "None"))
  (:Pressed
    (CallFunction|TeleporttoPoint (Variables|Cheats|Teleport|GetTeleportPoint5))))

(event Input|KeyboardEvents|NumPadSix
  (params (Key :type Key%20Structure :default "None"))
  (:Pressed
    (CallFunction|TeleporttoPoint (Variables|Cheats|Teleport|GetTeleportPoint6))))

(event Input|KeyboardEvents|NumPadSeven
  (params (Key :type Key%20Structure :default "None"))
  (:Pressed
    (CallFunction|TeleporttoPoint (Variables|Cheats|Teleport|GetTeleportPoint7))))

(event Input|KeyboardEvents|NumPadEight
  (params (Key :type Key%20Structure :default "None"))
  (:Pressed
    (CallFunction|TeleporttoPoint (Variables|Cheats|Teleport|GetTeleportPoint8))))

(event Input|KeyboardEvents|NumPadNine
  (params (Key :type Key%20Structure :default "None"))
  (:Pressed
    (CallFunction|TeleporttoPoint (Variables|Cheats|Teleport|GetTeleportPoint9))))

(fn ConstructionScript)

(fn InitCheatManager
  (params (EchoPlayerCharacter :type Character%20ST%20Object%20Reference) (EchoPlayerController :type Echo%20Player%20Controller%20Base%20Object%20Reference))
  (Variables|Cheats|SetEchoPlayerCharacter EchoPlayerCharacter)
  (bind _output_get (Variables|Cheats|SetEchoPlayerController EchoPlayerController))
  (Utilities|IsValid _output_get
    (:Is%20Valid
      (bind _returnvalue (UserInterface|CreateWidget "/Game/_ProjectEcho/Blueprints/UI/Cheat/WBP_CheatLoadScreen.WBP_CheatLoadScreen_C" (Variables|Cheats|GetEchoPlayerController)))
      (bind _output_get_2 (Variables|Cheats|SetLoadScreen _returnvalue))
      (Default|CEInit _output_get_2)
      (UserInterface|Viewport|AddtoViewport _output_get_2 0)
      (EventDispatchers|BindEventtoOnFadeinFinished _output_get_2 (EventDispatchers|CreateEvent :!event Custom|CE_OnLoadScreenFadeInFinished))
      (EventDispatchers|BindEventtoOnFadeOutFinished _output_get_2 (EventDispatchers|CreateEvent :!event Custom|CE_OnLoadScreenFadeOutFinished)))))
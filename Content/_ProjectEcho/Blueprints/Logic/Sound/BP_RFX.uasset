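; BP_RFX plays a recurring random sound effect at varying positions around the player.
; Its PlayRFX event waits a random time between MinRate and MaxRate, spawns the given sound, then calls itself again to loop indefinitely.
; X and Y offsets each get a random distance and sign, keeping sounds off the player, while height varies slightly.
; Nothing in this Blueprint starts the loop or stops it.
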(event Custom|PlayRFX
  (params (RFX :type Sound%20Base%20Object%20Reference) (MinRate :type Float%20%28double-precision%29) (MaxRate :type Float%20%28double-precision%29) (MinDistance :type Float%20%28double-precision%29) (MaxDistance :type Float%20%28double-precision%29))
  ;[0.2612 0.599 0.3442 0.5] Random delay
  (Utilities|FlowControl|Delay (Math|Random|RandomFloatinRange MinRate MaxRate))
  (Audio|SpawnSoundatLocation RFX (+ (Transformation|GetActorLocation (Variables|Default|GetPlayer)) (Math|Vector|MakeVector (* (Math|Random|RandomFloatinRange MinDistance MaxDistance) (Math|Integer|SelectInt -1 1 (Math|Random|RandomBool))) (* (Math|Random|RandomFloatinRange MinDistance MaxDistance) (Math|Integer|SelectInt -1 1 (Math|Random|RandomBool))) (Math|Random|RandomFloatinRange -1e+02 1e+02))) "0, 0, 0" 1.0 1.0 0.0 0 0)
  (CallFunction|PlayRFX RFX MinRate MaxRate MinDistance MaxDistance))

(fn ConstructionScript)
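; BP_AmbianceManager starts a level's ambient soundscape on BeginPlay, combining a 2D bed sound with a set of RFX sounds.
; For each entry in its RFX list, it looks up a DT_Rfx row and spawns a BPRFX actor at its own transform.
; Each spawned actor receives the player pawn, then plays the row's MetaSound using that row's rate and distance ranges.
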(event EventBeginPlay
  (Variables|Default|SetPlayer (Game|Player|GetPlayerPawn 0))
  ;[0.2612 0.599 0.3442 0.5] Play BED
  (Audio|SpawnSound2D (Variables|Default|GetBED) 1.0 1.0 0.0 0)
  ;[0.9375 0.1367 0.713 0.5] Spawn and play specified RFX
  (for _array_element (Variables|Default|GetRFX)
    (bind _returnvalue (Utilities|GetDataTableRow "/Game/_ProjectEcho/Assets/Audio/Data/DT_Rfx.DT_Rfx" (.RowName (Utilities|Struct|BreakDataTableRowHandle _array_element)))
      (:then
        (bind _returnvalue_2 (Game|SpawnActorfromClass (Variables|Default|GetBP_RFX) (Transformation|GetActorTransform) "Undefined" "MultiplyWithRoot" 0 0))
        (Variables|/Game/_ProjectEcho/Blueprints/Logic/Sound/BP_RFX.BP_RFX_C|SetPlayer _returnvalue_2 (Variables|Default|GetPlayer))
        (Default|PlayRFX _returnvalue_2 (.Metasound (Utilities|Struct|BreakStr_Rfx _returnvalue)) (.MinRate (Utilities|Struct|BreakStr_Rfx _returnvalue)) (.MaxRate (Utilities|Struct|BreakStr_Rfx _returnvalue)) (.MinDistance (Utilities|Struct|BreakStr_Rfx _returnvalue)) (.MaxDistance (Utilities|Struct|BreakStr_Rfx _returnvalue)))))))

(fn ConstructionScript)
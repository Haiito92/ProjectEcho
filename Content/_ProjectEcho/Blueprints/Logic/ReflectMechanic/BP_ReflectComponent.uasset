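; BP_ReflectComponent is a reflect-mechanic component that drives a Niagara effect from a list of predicted path positions.
; TryReflect pushes the positions into the system's vector and position arrays, and only when the point count changes updates PositionsCount, restarts the system and prints the count.
; StartReflect resets and activates the effect, and StopReflect deactivates it.
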(event EventBeginPlay)

(event EventTick
  (params (DeltaSeconds :type Float%20%28single-precision%29)))

(event EventTryReflect
  (params (PredictPathPositions :type Array%20of%20Vectors))
  (bind _returnvalue (Utilities|Array|Length PredictPathPositions))
  (bind _niagarasystem (Variables|Default|GetNiagaraSystem))
  (bind _niagarasystem_2 (Variables|Default|GetNiagaraSystem))
  (Utilities|IsValid _niagarasystem
    (:Is%20Valid
      (Class|NiagaraDataInterfaceArrayFunctionLibrary|SetNiagaraArrayVector _niagarasystem "Positions" PredictPathPositions)
      (Class|NiagaraDataInterfaceArrayFunctionLibrary|SetNiagaraArrayPosition _niagarasystem "Position Array" PredictPathPositions)
      (if (!= _returnvalue (Variables|Default|GetCount))
        (Class|NiagaraComponent|SetVariableInt _niagarasystem "PositionsCount" _returnvalue)
        (Variables|Default|SetCount _returnvalue)
        (Niagara|ResetSystem _niagarasystem_2)
        (Components|Activation|SetActive _niagarasystem_2 true false)
        (Development|PrintString (Utilities|String|ToString(Integer) _returnvalue))))))

(event EventStartReflect
  (bind _niagarasystem (Variables|Default|GetNiagaraSystem))
  (Utilities|IsValid _niagarasystem
    (:Is%20Valid
      (Niagara|ResetSystem _niagarasystem)
      (Components|Activation|Activate _niagarasystem true))))

(event EventStopReflect
  (bind _niagarasystem (Variables|Default|GetNiagaraSystem))
  (Utilities|IsValid _niagarasystem
    (:Is%20Valid
      (Components|Activation|Deactivate _niagarasystem))))
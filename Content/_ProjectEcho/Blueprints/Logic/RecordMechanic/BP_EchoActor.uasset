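; Echo actor for the record mechanic, replaying action, animation and control-rotation keys as a colored echo.
; Action keys drive interact, grab, propulse and reflect components, aimed by an Arrow that holds the control rotation.
; Animation keys feed the echo's anim blueprint, and InitEcho shows the meshes matching its color.
; Rewind and timeline destruction stop active abilities; jump, trace-detected landing, presence and rewind sounds attach to the mesh.
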(event Custom|ManuallySetControlRotation
  (params (Control%20Rotation :type Rotator))
  (Transformation|SetWorldRotation (Variables|Components|GetArrow) Control%20Rotation false false))

(event EventHandleActionKey
  (params (Action :type ERecordedAction%20Enum :default "None"))
  (bind _grabbing (Variables|Components|GetGrabbing))
  (bind _bp_reflectcomponent (Variables|Default|GetBP_ReflectComponent))
  (bind _arrow (Variables|Components|GetArrow))
  (bind _arrow_2 (Variables|Components|GetArrow))
  (bind _arrow_3 (Variables|Components|GetArrow))
  (bind _bp_propulsecomponent (Variables|Default|GetBP_PropulseComponent))
  (bind _grabbing_2 (Variables|Components|GetGrabbing))
  (bind _returnvalue (Transformation|GetWorldRotation _arrow))
  (switch Utilities|FlowControl|Switch|SwitchonERecordedAction Action
    (:Jump
      (if (not (Variables|Default|GetIsInRewind))
        ;[0.9375 0.1367 0.713 0.5] Jump sfx
        (Audio|SpawnSoundAttached "/Game/_ProjectEcho/Assets/Audio/MSSource/ECHOES/FT/Jump/MSS_ECHOES_FT_Jump_Concrete.MSS_ECHOES_FT_Jump_Concrete" (Variables|Default|GetEchoMesh) "None" "0, 0, 0" "0, 0, 0" "KeepRelativeOffset" false 1.0 1.0 0.0 0 0)))
    (:Interact
      (Class|Interactor|TryInteract (Variables|Default|GetInteractor) (Transformation|GetWorldLocation _arrow_3) (Math|Vector|GetForwardVector (Transformation|GetWorldRotation _arrow_3))))
    (:TryGrab
      (Class|GrabbingComponent|TryGrab _grabbing_2 _returnvalue (Utilities|Struct|MakeGrabbingRules "ECC_WorldStatic")))
    (:TryRelease
      (Class|GrabbingComponent|TryRelease _grabbing_2))
    (:TryThrow
      (Class|GrabbingComponent|TryThrow _grabbing_2 _returnvalue))
    (:TryPropulse
      (Class|PropulseComponent|TryPropulse _bp_propulsecomponent))
    (:StartPropulse
      (Class|PropulseComponent|StartPropulse _bp_propulsecomponent))
    (:StopPropulse
      (Class|PropulseComponent|StopPropulse _bp_propulsecomponent))
    (:StartReflect
      (Class|EchoDebug|AddonScreenDebugMessage "Reflect" "Log" "Echo Reflect" "(R=0.914080,G=1.000000,B=0.000000,A=1.000000)" 3.0)
      (Class|ReflectComponent|StartReflect _bp_reflectcomponent (Transformation|GetWorldLocation _arrow_2) (Math|Vector|GetForwardVector (Transformation|GetWorldRotation _arrow_2))))
    (:StopReflect
      (Class|ReflectComponent|StopReflect _bp_reflectcomponent))
    (:ForceGrab
      (Class|GrabbingComponent|TryForceGrabHeldCube _grabbing (Utilities|Struct|MakeGrabbingRules "ECC_WorldStatic")))
    (:ForceRelease
      (Class|GrabbingComponent|ForceRelease _grabbing))))

(event EventSetControlRotation
  (params (ControlRotation :type Rotator%20%28by%20ref%29 :default "0, 0, 0"))
  (Transformation|SetWorldRotation (Variables|Components|GetArrow) ControlRotation false false))

(event EventInitEcho
  (params (EchoColor :type Echo%20Color%20Struct%20Structure))
  (CallFunction|ActivateStaticMeshfromIndex (.colorenum EchoColor))
  ;[0.9375 0.1367 0.713 0.5] constant presence SFX
  (Audio|SpawnSoundAttached "/Game/_ProjectEcho/Assets/Audio/MSSource/ECHOES/MSS_ECHOES_Presence_LP.MSS_ECHOES_Presence_LP" (Variables|Default|GetEchoMesh) "None" "0, 0, 0" "0, 0, 0" "KeepRelativeOffset" false 1.0 1.0 0.0 0 0))

(event EventHandleRewindStarted
  (params (CurrentTimeKey :type Float%20%28single-precision%29%20%28by%20ref%29))
  ;[0.15 0.15 0.15 0.5] Handle Rewind
  (Class|PropulseComponent|StopPropulse (Variables|Default|GetBP_PropulseComponent))
  (Class|ReflectComponent|StopReflect (Variables|Default|GetBP_ReflectComponent))
  (Variables|Default|SetIsInRewind true)
  ;;[0.9375 0.1367 0.713 0.5] Rewind SFX
  (bind _returnvalue (Audio|SpawnSoundAttached "/Game/_ProjectEcho/Assets/Audio/MSSource/ECHOES/MSS_ECHOES_Rewind_LP.MSS_ECHOES_Rewind_LP" (Variables|Default|GetEchoMesh) "None" "0, 0, 0" "0, 0, 0" "KeepRelativeOffset" false 1.0 1.0 0.0 0 0))
  (Variables|Default|SetRewindLP _returnvalue))

(event EventHandleRewindStopped
  (params (CurrentTimeKey :type Float%20%28single-precision%29%20%28by%20ref%29))
  (bind _rewindlp (Variables|Default|GetRewindLP))
  ;[0.15 0.15 0.15 0.5] Handle Rewind
  (Variables|Default|SetIsInRewind false)
  ;;[0.9375 0.1367 0.713 0.5] Rewind SFX
  (Audio|SpawnSoundAttached "/Game/_ProjectEcho/Assets/Audio/MSSource/ECHOES/MSS_ECHOES_Rewind_Stop.MSS_ECHOES_Rewind_Stop" (Variables|Default|GetEchoMesh) "None" "0, 0, 0" "0, 0, 0" "KeepRelativeOffset" false 1.0 1.0 0.0 0 0)
  (Utilities|IsValid _rewindlp
    (:Is%20Valid
      (Class|AudioParameterControllerInterface|SetTriggerParameter _rewindlp "Stop"))))

(event EventOnTimelineDestroyed
  ;[0.15 0.15 0.15 0.5] Handle Timeline Destroyed
  (Class|GrabbingComponent|ForceRelease (Variables|Components|GetGrabbing))
  (Class|PropulseComponent|StopPropulse (Variables|Default|GetBP_PropulseComponent))
  (Class|ReflectComponent|StopReflect (Variables|Default|GetBP_ReflectComponent)))

(event EventTick
  (params (DeltaSeconds :type Float%20%28single-precision%29))
  (bind _arrow (Variables|Components|GetArrow))
  (bind _echomesh (Variables|Default|GetEchoMesh))
  (bind _returnvalue (Transformation|GetWorldLocation _echomesh))
  (Utilities|FlowControl|Sequence
    (:then_0
      ;[0.15 0.15 0.15 0.5] Tick of for Reflect Component
      (if (Class|ReflectComponent|Ison (Variables|Default|GetBP_ReflectComponent))
        (Class|ReflectComponent|SetCastStartLocation (Variables|Default|GetBP_ReflectComponent) (Transformation|GetWorldLocation _arrow))
        (Class|ReflectComponent|SetCastDirection (Variables|Default|GetBP_ReflectComponent) (Math|Vector|GetForwardVector (Transformation|GetWorldRotation _arrow)))))
    (:then_1
      (if (not (Variables|Default|GetIsInRewind))
        ;[0.9375 0.1367 0.713 0.5] Land SFX
        (bind _returnvalue_2 (Collision|LineTraceByChannel _returnvalue (- _returnvalue "0.000000,0.000000,150.000000") "TraceTypeQuery1" false 0 "None"))
        (if _returnvalue_2
          (Utilities|FlowControl|DoOnce false :!label _label
            (:Completed
              (Audio|SpawnSoundAttached "/Game/_ProjectEcho/Assets/Audio/MSSource/ECHOES/FT/Land/MSS_ECHOES_FT_Land_Concrete.MSS_ECHOES_FT_Land_Concrete" (Variables|Default|GetEchoMesh) "None" "0, 0, 0" "0, 0, 0" "KeepRelativeOffset" false 1.0 1.0 0.0 0 0)))
          (else
            (goto _label Reset)))))))

(event EventHandleAnimationBooleanKey
  (params (AnimationValue :type EAnimationValueReference%20Enum :default "None") (Value :type Boolean))
  (Default|ReceiveBoolAnim (Variables|Default|GetEcho%20Read%20Data) AnimationValue Value))

(event EventHandleAnimationFloatKey
  (params (AnimationValue :type EAnimationValueReference%20Enum :default "None") (Value :type Float%20%28single-precision%29))
  (Default|ReceiveFloatAnim (Variables|Default|GetEcho%20Read%20Data) AnimationValue Value))

(event EventBeginPlay
  (CallFunction|GetAnimationBlueprint))

(fn ConstructionScript)

(fn GetEchoControlRotation
  (return (Transformation|GetWorldRotation (Variables|Components|GetArrow))))

(fn ActivateStaticMeshfromIndex
  (params (Color :type EEchoColor%20Enum :default "Blue"))
  (for _array_element (Utilities|Array|MakeArray (Variables|Default|GetBlue1) (Variables|Default|GetBlue2) (Variables|Default|GetBlue3) (Variables|Default|GetRed1) (Variables|Default|GetRed2) (Variables|Default|GetGreen1) (Variables|Default|GetGreen2) (Variables|Default|GetYellow2) (Variables|Default|GetYellow3) (Variables|Default|GetYellow1))
    (Development|SetHiddeninGame _array_element (not (Utilities|Array|ContainsItem (Utilities|Select :Index Color :Blue (Utilities|Array|MakeArray (Variables|Default|GetBlue1) (Variables|Default|GetBlue2) (Variables|Default|GetBlue3)) :Red (Utilities|Array|MakeArray (Variables|Default|GetRed1) (Variables|Default|GetRed2)) :Green (Utilities|Array|MakeArray (Variables|Default|GetGreen1) (Variables|Default|GetGreen2)) :Yellow (Utilities|Array|MakeArray (Variables|Default|GetYellow2) (Variables|Default|GetYellow3) (Variables|Default|GetYellow1)) :Purple 0) _array_element)) false)))

(fn GetAnimationBlueprint
  (bind _asabp_echo_read_data (Utilities|Casting|CastToABP_Echo_Read_Data (Components|SkeletalMesh|GetAnimInstance (Variables|Default|GetEchoMesh))))
  (Variables|Default|SetEcho%20Read%20Data _asabp_echo_read_data))

(fn GetRecorderTimelineIndex
  (return (Variables|Default|GetEchoIndex)))

(fn ShouldRecord
  (return true))
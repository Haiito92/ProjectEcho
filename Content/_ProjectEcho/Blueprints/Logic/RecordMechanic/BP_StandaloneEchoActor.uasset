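; BP_StandaloneEchoActor is an actor in the record mechanic that opts out of recording.
; ShouldRecord and ShouldInteractionListenForRecord both return false, so it neither records nor has its interaction listen for recording.
; A Look At Help Sphere function rotates the Arrow component to face the HelpSphere component.
; The event graph holds only disabled stubs, and construction defers to the parent.
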(event EventBeginPlay)

(event Collision|EventActorBeginOverlap
  (params (OtherActor :type Actor%20Object%20Reference)))

(event EventTick
  (params (DeltaSeconds :type Float%20%28single-precision%29))
  (|CallParentFunction DeltaSeconds) ; This node is disabled and will not be called.\nDrag off pins to build functionality.
)

(fn ConstructionScript
  (|CallParentFunction))

(fn LookatHelpSphere
  (bind _arrow (Variables|Default|GetArrow))
  (Transformation|SetWorldRotation _arrow (Math|Rotator|FindLookatRotation (Transformation|GetWorldLocation _arrow) (Transformation|GetWorldLocation (Variables|Default|GetHelpSphere))) false false))

(fn ShouldRecord
  (return false))

(fn ShouldInteractionListenforRecord
  (return false))
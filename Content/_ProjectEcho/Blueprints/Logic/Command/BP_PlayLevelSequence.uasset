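; Command Blueprint that plays a configurable level sequence when executed.
; It creates a level sequence player at runtime with the configured loop count and no autoplay, then starts playback immediately.
; For loop counts above -1, it sets the spawned sequence actor's lifespan to loop count times sequence duration in seconds, for automatic cleanup.
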(event EventReceiveExecute
  (params (Context :type Command%20Context%20Structure%20%28by%20ref%29))
  (bind _loopcount (Variables|Default|GetLoopCount))
  (bind (_outactor _returnvalue) (Sequencer|Player|CreateLevelSequencePlayer self (Variables|Default|GetLevelSequence) (Utilities|Struct|MakeMovieSceneSequencePlaybackSettings false (Utilities|Struct|MakeMovieSceneSequenceLoopCount (Variables|Default|GetLoopCount)))))
  (Sequencer|Player|Play _returnvalue :!class /Script/MovieScene.MovieSceneSequencePlayer)
  (if (> _loopcount -1)
    (Actor|SetLifeSpan _outactor (* _loopcount (Class|TimeManagementBlueprintLibrary|ToSeconds(QualifiedFrameTime) (Media|MediaPlayer|GetDuration _returnvalue))))))
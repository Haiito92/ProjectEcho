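; BP_CommandTriggerBox is a trigger volume that runs configurable command lists when the Echo player enters or leaves its box.
; Begin and end overlaps ignore any actor that fails the cast to BPC_EchoPlayer.
; Each event first executes its one-time command list through a DoOnce that is never reset, then its repeatable list on every overlap.
; All lists execute through ExecuteCommandsWithContext, with the trigger itself as instigator.
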(event OnComponentBeginOverlap(Box)
  (params (OverlappedComponent :type Primitive%20Component%20Object%20Reference) (OtherActor :type Actor%20Object%20Reference) (OtherComp :type Primitive%20Component%20Object%20Reference) (OtherBodyIndex :type Integer) (bFromSweep :type Boolean) (SweepResult :type Hit%20Result%20Structure%20%28by%20ref%29))
  (Utilities|Casting|CastToBPC_EchoPlayer OtherActor)
  (Utilities|FlowControl|Sequence
    (:then_0
      (Utilities|FlowControl|DoOnce false
        (:Completed
          (Class|CommandFunctionLibrary|ExecuteCommandswithContext (Variables|Commands|Once|GetDoneOnceBeginOverlapCommands) self))))
    (:then_1
      (Class|CommandFunctionLibrary|ExecuteCommandswithContext (Variables|Commands|Always|GetBeginOverlapCommands) self))))

(event OnComponentEndOverlap(Box)
  (params (OverlappedComponent :type Primitive%20Component%20Object%20Reference) (OtherActor :type Actor%20Object%20Reference) (OtherComp :type Primitive%20Component%20Object%20Reference) (OtherBodyIndex :type Integer))
  (Utilities|Casting|CastToBPC_EchoPlayer OtherActor)
  (Utilities|FlowControl|Sequence
    (:then_0
      (Utilities|FlowControl|DoOnce false
        (:Completed
          (Class|CommandFunctionLibrary|ExecuteCommandswithContext (Variables|Commands|Once|GetDoneOnceEndOverlapCommands) self))))
    (:then_1
      (Class|CommandFunctionLibrary|ExecuteCommandswithContext (Variables|Commands|Always|GetEndOverlapCommands) self))))

(fn ConstructionScript)
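; Test actor for the activable mechanic that acts as an interactable switch.
; Its switch on, off and toggle events forward to a BPActivatorComponent.
; Interacting prints an on-screen debug message and toggles the switch.
; IsSwitchOn is a stub that always returns false rather than reading the component's state.
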(event EventInteract
  (Class|EchoDebug|AddonScreenDebugMessage "Interact" "Log" "I was interacted with" "(R=0.000000,G=1.000000,B=0.543633,A=1.000000)" 3.0)
  (Class|Activator|ToggleSwitch))

(event EventSwitchon
  (Class|Activator|Switchon (Variables|Default|GetBP_ActivatorComponent)))

(event EventSwitchOff
  (Class|Activator|SwitchOff (Variables|Default|GetBP_ActivatorComponent)))

(event EventToggleSwitch
  (Class|Activator|ToggleSwitch (Variables|Default|GetBP_ActivatorComponent)))

(fn ConstructionScript)

(fn IsSwitchon
  (return false))
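; Tutorial trigger actor that plays a 2D sound and shows a UI widget the first time the player enters its box.
; The box overlap only responds to BPC_EchoPlayer and is gated by a DoOnce.
; With HasSound set, it plays the sound and, if HasWBP is also set, waits for the sound's duration before adding the widget to the viewport.
; Without a sound, it adds the widget immediately, skipping the HasWBP check.
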(event OnComponentBeginOverlap(Box)
  (params (OverlappedComponent :type Primitive%20Component%20Object%20Reference) (OtherActor :type Actor%20Object%20Reference) (OtherComp :type Primitive%20Component%20Object%20Reference) (OtherBodyIndex :type Integer) (bFromSweep :type Boolean) (SweepResult :type Hit%20Result%20Structure%20%28by%20ref%29))
  (bind _sound (Variables|Default|GetSound))
  (Utilities|Casting|CastToBPC_EchoPlayer OtherActor)
  (Utilities|FlowControl|DoOnce false
    (:Completed
      (if (Variables|Default|GetHasSound?)
        (Audio|PlaySound2D _sound 1.0 1.0 0.0 0 0)
        (if (Variables|Default|GetHasWBP?)
          (Utilities|FlowControl|Delay (Variables|/Script/Engine.SoundBase|GetDuration _sound))
          (bind _returnvalue (UserInterface|CreateWidget (Utilities|GetClass (Variables|Default|GetWidgetToSpaw)) :!label _label))
          (UserInterface|Viewport|AddtoViewport _returnvalue 0))
        (else
          (goto _label))))))

(event EventBeginPlay)

(fn ConstructionScript)
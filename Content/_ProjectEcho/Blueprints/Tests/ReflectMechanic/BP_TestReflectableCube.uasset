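; Test physics cube for the reflect mechanic that always reports itself as reflectable.
; On Reflect it gets a velocity-change impulse along the given direction scaled by power, and logs the power and direction on screen.
; Hard enough hits play an attached wood impact sound with a randomised velocity parameter, throttled by a DoOnce that resets after a short random delay.
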(event OnComponentHit(Cube)
  (params (HitComponent :type Primitive%20Component%20Object%20Reference) (OtherActor :type Actor%20Object%20Reference) (OtherComp :type Primitive%20Component%20Object%20Reference) (NormalImpulse :type Vector :default "0, 0, 0") (Hit :type Hit%20Result%20Structure%20%28by%20ref%29))
  (bind _returnvalue (Transformation|GetVelocity))
  (bind _returnvalue_2 (Math|Vector|VectorLength _returnvalue))
  ;[0.9375 0.1367 0.713 0.5] Impact sfx
  ;;[0.2612 0.599 0.3442 0.5] Minimum velocity required
  (if (>= _returnvalue_2 2e+02)
    (Utilities|FlowControl|DoOnce false :!label _label
      (:Completed
        (bind _returnvalue_3 (Audio|SpawnSoundAttached "/Game/_ProjectEcho/Assets/Audio/MSSource/GPE/PhysicsObjects/Wood/MSS_GPE_PhysicsObjects_Wood.MSS_GPE_PhysicsObjects_Wood" (Variables|Default|GetCube) "None" "0, 0, 0" "0, 0, 0" "KeepRelativeOffset" false 1.0 1.0 0.0 0 0))
        (Audio|Parameter|SetFloatParameter _returnvalue_3 "Velocity" (+ _returnvalue_2 (Math|Random|RandomFloatinRange -5e+01 5e+01)) :!class /Script/AudioExtensions.AudioParameterControllerInterface)
        (Utilities|FlowControl|Delay (Math|Random|RandomFloatinRange 0.1 0.3))
        (goto _label Reset)))))

(event EventBeginPlay)

(event Collision|EventActorBeginOverlap
  (params (OtherActor :type Actor%20Object%20Reference)))

(event EventTick
  (params (DeltaSeconds :type Float%20%28single-precision%29)))

(event EventReflect
  (params (ReflectDirection :type Vector%20%28by%20ref%29 :default "0, 0, 0") (ReflectPower :type Float%20%28single-precision%29))
  (Utilities|FlowControl|Sequence
    (:then_0
      (Physics|AddImpulse (Variables|Default|GetCube) (* ReflectDirection ReflectPower) "None" true)
      (Class|EchoDebug|AddonScreenDebugMessage "Reflect" "Log" "TestCubeReflect" "(R=0.191023,G=0.294890,B=1.000000,A=1.000000)" 3.0))
    (:then_1
      (Class|EchoDebug|AddonScreenDebugMessage "Reflect" "Log" (Utilities|String|ToString(Float) ReflectPower) "(R=0.191023,G=0.294890,B=1.000000,A=1.000000)" 3.0)
      (Class|EchoDebug|AddonScreenDebugMessage "Reflect" "Log" (Utilities|String|ToString(Vector) ReflectDirection) "(R=0.191023,G=0.294890,B=1.000000,A=1.000000)" 3.0))))

(fn ConstructionScript)

(fn CanbeReflected
  (return true))